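; BP_Kiosk is a kiosk actor that spawns an instance of SpawningClass when its ShelfVolume is hit.
; The spawn point is offset from the impact point by a random distance, pointing away from a random point inside SpawningVolume, and ignores collision.
; A DoOnce limits this to one spawn until any overlap with WalkwayVolume ends, which re-arms it.
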(event OnComponentEndOverlap(WalkwayVolume)
  (params (OtherActor :type Actor%20Object%20Reference) (OtherComp :type Primitive%20Component%20Object%20Reference) (OtherBodyIndex :type Integer))
  (bind _spawning_volume (Variables|Default|GetSpawning%20Volume))
  (Utilities|FlowControl|DoOnce false) ; enters at Reset
)

(event OnComponentHit(ShelfVolume)
  (params (OtherActor :type Actor%20Object%20Reference) (OtherComp :type Primitive%20Component%20Object%20Reference) (NormalImpulse :type Vector) (Hit :type Hit%20Result%20Structure%20%28by%20ref%29))
  (bind _impactpoint (Collision|BreakHitResult Hit))
  (bind _spawning_volume (Variables|Default|GetSpawning%20Volume))
  (Utilities|FlowControl|DoOnce false
    (:Completed
      (Game|SpawnActorfromClass (Variables|Default|GetSpawning%20Class) (Math|Transform|MakeTransform (+ _impactpoint (* (Math|Vector|Normalize (- _impactpoint (Math|Random|RandomPointinBoundingBox (Transformation|GetWorldLocation _spawning_volume) (Components|Box|GetScaledBoxExtent _spawning_volume)))) (Math|Random|RandomFloatinRange 0.0 1e+02)))) "AlwaysSpawn" 0 0))))

(fn ConstructionScript)