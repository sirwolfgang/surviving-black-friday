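; Front door Blueprint that opens when something overlaps its trigger collision and closes after it leaves.
; BeginPlay caches both doors' relative start locations; overlap begin plays a timeline, and overlap end reverses it after a short delay.
; The timeline's vector track offsets the right door from its start, while the left door's lerp has zero alpha, so it stays in place.
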(event OnComponentBeginOverlap(OpenDoorCollision)
  (params (OtherActor :type Actor%20Object%20Reference) (OtherComp :type Primitive%20Component%20Object%20Reference) (OtherBodyIndex :type Integer) (bFromSweep :type Boolean) (SweepResult :type Hit%20Result%20Structure%20%28by%20ref%29))
  ;[1 1 1] OpenDoor
  (bind _doorlocation (Timeline|Timeline_DoorOpenClose Play)
    (:Update
      (Transformation|SetRelativeLocation (Variables|Default|GetDoorLeft) (Math|Vector|Lerp(Vector) (Variables|Default|GetL_DoorStart) _doorlocation 0.0) false false)
      (Transformation|SetRelativeLocation (Variables|Default|GetDoorRight) (+ (Variables|Default|GetR_DoorStart) _doorlocation) false false))))

(event OnComponentEndOverlap(OpenDoorCollision)
  (params (OtherActor :type Actor%20Object%20Reference) (OtherComp :type Primitive%20Component%20Object%20Reference) (OtherBodyIndex :type Integer))
  ;[1 1 1] CloseDoor
  (Utilities|FlowControl|Delay 0.5)
  (bind _doorlocation (Timeline|Timeline_DoorOpenClose Reverse)
    (:Update
      (Transformation|SetRelativeLocation (Variables|Default|GetDoorLeft) (Math|Vector|Lerp(Vector) (Variables|Default|GetL_DoorStart) _doorlocation 0.0) false false)
      (Transformation|SetRelativeLocation (Variables|Default|GetDoorRight) (+ (Variables|Default|GetR_DoorStart) _doorlocation) false false))))

(event EventBeginPlay
  ;[1 1 1] Set Door Initial Location
  (Variables|Default|SetL_DoorStart (Variables|/Script/Engine.SceneComponent|GetRelativeLocation (Variables|Default|GetDoorLeft)))
  (Variables|Default|SetR_DoorStart (Variables|/Script/Engine.SceneComponent|GetRelativeLocation (Variables|Default|GetDoorRight))))

(fn ConstructionScript)