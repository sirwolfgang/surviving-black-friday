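; BP_Shelf_Pack_Box is a prefab of nine box components, named as a shelf pack, that gets a random color when play begins.
; BeginPlay creates one dynamic material instance from Box_Mat_Base and sets its BaseColor parameter to random RGB values with full alpha.
; All nine boxes share that instance, so each pack has a single color and the color is not set in the construction script.
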(event EventBeginPlay
  (bind _returnvalue (Rendering|Material|CreateDynamicMaterialInstance "/Game/Meshes/Materials/Box_Mat_Base.Box_Mat_Base" :!class /Script/Engine.KismetMaterialLibrary))
  (Rendering|Material|SetVectorParameterValue _returnvalue "BaseColor" (Utilities|Struct|MakeLinearColor (Math|Random|RandomFloatinRange 0.0 1.0) (Math|Random|RandomFloatinRange 0.0 1.0) (Math|Random|RandomFloatinRange 0.0 1.0) 1.0) :!class /Script/Engine.MaterialInstanceDynamic)
  (Rendering|Material|SetMaterial (Variables|Default|GetBox%201) 0 _returnvalue))

(fn ConstructionScript)