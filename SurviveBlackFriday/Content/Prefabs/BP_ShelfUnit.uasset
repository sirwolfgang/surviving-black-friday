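; BP_ShelfUnit is a store shelf that spawns pack boxes on three levels at BeginPlay and displays a random item component's sale price.
; The price text shifts from white toward yellow with the item's value.
; A hit on the shelf spawns a SpawningClass actor near the impact once, re-armed when a WalkwayVolume overlap ends.
; Tick clears the custom-depth glow every frame, so highlighting must be re-applied externally.
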(event OnComponentEndOverlap(WalkwayVolume)
  (params (OtherActor :type Actor%20Object%20Reference) (OtherComp :type Primitive%20Component%20Object%20Reference) (OtherBodyIndex :type Integer))
  (bind _spawning_volume (Variables|Default|GetSpawning%20Volume))
  (Utilities|FlowControl|DoOnce false) ; enters at Reset
)

(event OnComponentHit(ShelfVolume)
  (params (OtherActor :type Actor%20Object%20Reference) (OtherComp :type Primitive%20Component%20Object%20Reference) (NormalImpulse :type Vector) (Hit :type Hit%20Result%20Structure%20%28by%20ref%29))
  (bind _impactpoint (Collision|BreakHitResult Hit))
  (bind _spawning_volume (Variables|Default|GetSpawning%20Volume))
  (Utilities|FlowControl|DoOnce false
    (:Completed
      (Game|SpawnActorfromClass (Variables|Default|GetSpawning%20Class) (Math|Transform|MakeTransform (+ _impactpoint (* (Math|Vector|Normalize (- _impactpoint (Math|Random|RandomPointinBoundingBox (Transformation|GetWorldLocation _spawning_volume) (Components|Box|GetScaledBoxExtent _spawning_volume)))) (Math|Random|RandomFloatinRange 0.0 1e+02)))) "AlwaysSpawn" 0 0))))

(event EventBeginPlay
  (bind _returnvalue (Actor|GetComponentsByClass "/Game/Prefabs/Items/Item_Blueprint.Item_Blueprint_C"))
  (bind _textrender (Variables|Default|GetTextRender))
  (Game|SpawnActorfromClass "/Game/Prefabs/BP_Shelf_Pack_Box.BP_Shelf_Pack_Box_C" (Transformation|GetWorldTransform (Variables|Default|GetShelf%20Pack%20Zone%20Top)) "AlwaysSpawn" 0 0)
  (Game|SpawnActorfromClass "/Game/Prefabs/BP_Shelf_Pack_Box.BP_Shelf_Pack_Box_C" (Transformation|GetWorldTransform (Variables|Default|GetShelf%20Pack%20Zone%20Middle)) "AlwaysSpawn" 0 0)
  (Game|SpawnActorfromClass "/Game/Prefabs/BP_Shelf_Pack_Box.BP_Shelf_Pack_Box_C" (Transformation|GetWorldTransform (Variables|Default|GetShelf%20Pack%20Zone%20Bottom)) "AlwaysSpawn" 0 0)
  (bind _output_get (Variables|Default|SetItemOnShelf (Utilities|Array|Get(acopy) _returnvalue (Math|Random|RandomInteger (Utilities|Array|Length _returnvalue)))))
  ;[1 1 1] Setup Text Renderer
  (Rendering|Components|TextRender|SetText _textrender (Utilities|Text|ToText(Integer) (Variables|/Game/Prefabs/Items/Item_Blueprint.Item_Blueprint_C|GetSalePrice _output_get)))
  (Rendering|Components|TextRender|SetTextRenderColor _textrender (Math|Conversions|ToColor(LinearColor) (Math|Color|Lerp(LinearColor) "(R=1.000000,G=1.000000,B=1.000000,A=1.000000)" "(R=1.000000,G=1.000000,B=0.000000,A=1.000000)" (/ (Math|Conversions|ToFloat(Integer) (Variables|/Game/Prefabs/Items/Item_Blueprint.Item_Blueprint_C|GetValue _output_get)) 5e+02)))))

(event EventTick
  (params (DeltaSeconds :type Float%20%28single-precision%29))
  (bind _singlesideshelf (Variables|Default|GetSingleSideShelf))
  ;[1 1 1] Removes custom depth post processing for shelf glow if glowing at begin of tick
  (if (Variables|/Script/Engine.PrimitiveComponent|GetbRenderCustomDepth _singlesideshelf)
    (Rendering|SetRenderCustomDepth _singlesideshelf false)))

(fn ConstructionScript)