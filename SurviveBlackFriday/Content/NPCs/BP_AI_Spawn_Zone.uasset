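; BP_AI_Spawn_Zone is a spawn volume that populates its area with AI NPCs when play begins.
; It spawns SpawnCount pawns at random points within the SpawnZone component's bounds, picking each class from the first six entries of AICharacterArray.
; Each pawn runs Base_AI_BT and receives the zone's NavigationData object through its "Navigation Data" blackboard key.
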(event EventBeginPlay
  (bind _spawn_zone (Variables|Default|GetSpawn%20Zone))
  (bind (_origin _boxextent) (Collision|GetComponentBounds _spawn_zone))
  (for _index (range 0 (Variables|Default|GetSpawn%20Count))
    (bind _returnvalue (AI|SpawnAIFromClass (Utilities|Array|Get(acopy) (Variables|Default|GetAICharacterArray) (Math|Random|RandomInteger 6)) "/Game/NPCs/Base_AI_BT.Base_AI_BT" (Math|Random|RandomPointinBoundingBox _origin _boxextent) "0, 0, 0" false))
    (AI|Components|Blackboard|SetValueasObject (AI|GetBlackboard _returnvalue) (Utilities|Name|MakeLiteralName "Navigation Data") (Variables|Default|GetNavigation%20Data))))

(fn ConstructionScript)